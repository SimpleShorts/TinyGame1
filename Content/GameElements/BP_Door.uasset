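; BP_Door is a sliding door that opens and closes in response to an interaction on a separate trigger actor.
; On BeginPlay it binds to the OnInteract event of the BP_InteractionComponent on its Trigger reference, if both are valid.
; The event's On flag plays or reverses the DoorAnimation timeline, which offsets both door meshes along their relative Y axis.
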(event Custom|OpenDoor
  (bind _doormovement (Timeline|DoorAnimation Play)
    (:Update
      (Transformation|SetRelativeLocation (Variables|Default|GetSM_Door_R) (Math|Vector|MakeVector 0.0 (* _doormovement -7e+01) 0.0) false false))))

(event Custom|CloseDoor
  (bind _doormovement (Timeline|DoorAnimation Reverse)
    (:Update
      (Transformation|SetRelativeLocation (Variables|Default|GetSM_Door_R) (Math|Vector|MakeVector 0.0 (* _doormovement -7e+01) 0.0) false false))))

(event Custom|OnInteract_Event_0
  (params (on :type Boolean))
  (if on
    (CallFunction|OpenDoor)
    (else
      (CallFunction|CloseDoor))))

(event EventBeginPlay
  (bind _trigger (Variables|Default|GetTrigger)
    (:then
      (Utilities|IsValid (Actor|GetComponentbyClass _trigger "/Game/Framework/BP_InteractionComponent.BP_InteractionComponent_C")
        (:Is%20Valid
          (EventDispatchers|AssignOnInteract (Actor|GetComponentbyClass _trigger "/Game/Framework/BP_InteractionComponent.BP_InteractionComponent_C") (delegate Custom|OnInteract_Event_0)))))
    (:else)))

(fn ConstructionScript)